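; Endless-runner scenery segment that fills itself with randomized buildings and triggers creation of the next segment.
; The construction script calls SpawnBuildings, which adds child actor components at the SP marker transforms, most chosen by random branch and two fixed.
; Overlapping its Box calls ExtendBuildings on BP_RunnerGameMode, without filtering the overlapping actor.
; GetAttachPoint returns the Arrow's world transform as an attachment point.
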(event `self.Box.OnComponentBeginOverlap`
  (params (OverlappedComponent :type "PrimitiveComponent Object Reference") (OtherActor :type "Actor Object Reference") (OtherComp :type "PrimitiveComponent Object Reference") (OtherBodyIndex :type Integer) (bFromSweep :type Boolean) (SweepResult :type "HitResult Structure (by ref)"))
  ;[1 1 1] Extend Buildings
  (bind _asbp_runner_game_mode (cast `/Game/Runner/Blueprints/BP_RunnerGameMode` (`GameplayStatics.GetGameMode`)))
  (`/Game/Runner/Blueprints/BP_RunnerGameMode.Extend Buildings` _asbp_runner_game_mode))

(fn `Get AttachPoint`
  (returns (ReturnValue :type "Transform Structure"))
  (return (`SceneComponent.K2_GetComponentToWorld` (`self.Arrow`))))

(fn `SpawnBuildings`
  (bind _returnvalue (`SceneComponent.GetRelativeTransform` (`self.SP12`)))
  (bind _returnvalue_2 (`SceneComponent.GetRelativeTransform` (`self.SP4`)))
  (bind _returnvalue_3 (`SceneComponent.GetRelativeTransform` (`self.SP5`)))
  (bind _returnvalue_4 (`SceneComponent.GetRelativeTransform` (`self.SP1`)))
  (bind _returnvalue_5 (`SceneComponent.GetRelativeTransform` (`self.SP2`)))
  (bind _returnvalue_6 (`SceneComponent.GetRelativeTransform` (`self.SP3`)))
  (bind _returnvalue_7 (`SceneComponent.GetRelativeTransform` (`self.SP8`)))
  (bind _returnvalue_8 (`SceneComponent.GetRelativeTransform` (`self.SP9`)))
  (bind _returnvalue_9 (`SceneComponent.GetRelativeTransform` (`self.SP11`)))
  (bind _returnvalue_10 (`SceneComponent.GetRelativeTransform` (`self.SP6`)))
  (`|ExecutionSequence`
    (:`then_0`
      (switch `int` (`KismetMathLibrary.RandomIntegerInRange` 0 3)
        (:`0`
          (`AddComponent|NODE_AddChildActorComponent-6` :`RelativeTransform` _returnvalue_4))
        (:`1`
          (`AddComponent|NODE_AddChildActorComponent-7` :`RelativeTransform` _returnvalue_4))
        (:`2`
          (`AddComponent|NODE_AddChildActorComponent-8` :`RelativeTransform` _returnvalue_4))
        (:`3`
          (`AddComponent|NODE_AddChildActorComponent-9` :`RelativeTransform` _returnvalue_4))))
    (:`then_1`
      (switch `int` (`KismetMathLibrary.RandomIntegerInRange` 0 3)
        (:`0`
          (`AddComponent|NODE_AddChildActorComponent-18` :`RelativeTransform` _returnvalue_5))
        (:`1`
          (`AddComponent|NODE_AddChildActorComponent-19` :`RelativeTransform` _returnvalue_5))
        (:`2`
          (`AddComponent|NODE_AddChildActorComponent-20` :`RelativeTransform` _returnvalue_5))
        (:`3`
          (`AddComponent|NODE_AddChildActorComponent-21` :`RelativeTransform` _returnvalue_5))))
    (:`then_2`
      (switch `int` (`KismetMathLibrary.RandomIntegerInRange` 0 3)
        (:`0`
          (`AddComponent|NODE_AddChildActorComponent-22` :`RelativeTransform` _returnvalue_6))
        (:`1`
          (`AddComponent|NODE_AddChildActorComponent-23` :`RelativeTransform` _returnvalue_6))
        (:`2`
          (`AddComponent|NODE_AddChildActorComponent-24` :`RelativeTransform` _returnvalue_6))
        (:`3`
          (`AddComponent|NODE_AddChildActorComponent-25` :`RelativeTransform` _returnvalue_6))))
    (:`then_3`
      (switch `int` (`KismetMathLibrary.RandomIntegerInRange` 0 3)
        (:`0`
          (`AddComponent|NODE_AddChildActorComponent-34` :`RelativeTransform` _returnvalue_2))
        (:`1`
          (`AddComponent|NODE_AddChildActorComponent-35` :`RelativeTransform` _returnvalue_2))
        (:`2`
          (`AddComponent|NODE_AddChildActorComponent-36` :`RelativeTransform` _returnvalue_2))
        (:`3`
          (`AddComponent|NODE_AddChildActorComponent-37` :`RelativeTransform` _returnvalue_2))))
    (:`then_4`
      (switch `int` (`KismetMathLibrary.RandomIntegerInRange` 0 3)
        (:`0`
          (`AddComponent|NODE_AddChildActorComponent-30` :`RelativeTransform` _returnvalue_3))
        (:`1`
          (`AddComponent|NODE_AddChildActorComponent-31` :`RelativeTransform` _returnvalue_3))
        (:`2`
          (`AddComponent|NODE_AddChildActorComponent-32` :`RelativeTransform` _returnvalue_3))
        (:`3`
          (`AddComponent|NODE_AddChildActorComponent-33` :`RelativeTransform` _returnvalue_3))))
    (:`then_5`
      (switch `int` (`KismetMathLibrary.RandomIntegerInRange` 0 3)
        (:`0`
          (`AddComponent|NODE_AddChildActorComponent-26` :`RelativeTransform` _returnvalue_10))
        (:`1`
          (`AddComponent|NODE_AddChildActorComponent-27` :`RelativeTransform` _returnvalue_10))
        (:`2`
          (`AddComponent|NODE_AddChildActorComponent-28` :`RelativeTransform` _returnvalue_10))
        (:`3`
          (`AddComponent|NODE_AddChildActorComponent-29` :`RelativeTransform` _returnvalue_10))))
    (:`then_6`
      (`AddComponent|NODE_AddChildActorComponent-38` :`RelativeTransform` (`SceneComponent.GetRelativeTransform` (`self.SP7`))))
    (:`then_7`
      (switch `int` (`KismetMathLibrary.RandomIntegerInRange` 0 2)
        (:`0`
          (`AddComponent|NODE_AddChildActorComponent-39` :`RelativeTransform` _returnvalue_7))
        (:`1`
          (`AddComponent|NODE_AddChildActorComponent-40` :`RelativeTransform` _returnvalue_7))
        (:`2`
          (`AddComponent|NODE_AddChildActorComponent-48` :`RelativeTransform` _returnvalue_7))))
    (:`then_8`
      (switch `int` (`KismetMathLibrary.RandomIntegerInRange` 0 2)
        (:`0`
          (`AddComponent|NODE_AddChildActorComponent-42` :`RelativeTransform` _returnvalue_8))
        (:`1`
          (`AddComponent|NODE_AddChildActorComponent-41` :`RelativeTransform` _returnvalue_8))
        (:`2`
          (`AddComponent|NODE_AddChildActorComponent-49` :`RelativeTransform` _returnvalue_8))))
    (:`then_9`
      (`AddComponent|NODE_AddChildActorComponent-43` :`RelativeTransform` (`SceneComponent.GetRelativeTransform` (`self.SP10`))))
    (:`then_10`
      (switch `int` (`KismetMathLibrary.RandomIntegerInRange` 0 2)
        (:`0`
          (`AddComponent|NODE_AddChildActorComponent-44` :`RelativeTransform` _returnvalue_9))
        (:`1`
          (`AddComponent|NODE_AddChildActorComponent-45` :`RelativeTransform` _returnvalue_9))
        (:`2`
          (`AddComponent|NODE_AddChildActorComponent-51` :`RelativeTransform` _returnvalue_9))))
    (:`then_11`
      (switch `int` (`KismetMathLibrary.RandomIntegerInRange` 0 2)
        (:`0`
          (`AddComponent|NODE_AddChildActorComponent-47` :`RelativeTransform` _returnvalue))
        (:`1`
          (`AddComponent|NODE_AddChildActorComponent-46` :`RelativeTransform` _returnvalue))
        (:`2`
          (`AddComponent|NODE_AddChildActorComponent-52` :`RelativeTransform` _returnvalue))))))

(fn `UserConstructionScript`
  (`self.SpawnBuildings`))