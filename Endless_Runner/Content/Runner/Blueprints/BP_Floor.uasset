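; BP_Floor is an endless-runner floor tile that populates itself with obstacles, coins and occasional power-ups.
; Its construction script builds per-lane arrow spawn points, shuffles them and attaches child actors, gating power-ups on the game mode's FloorCount, which it then resets.
; Box overlap asks BP_RunnerGameMode to extend the floor, raises player speed within a clamp and adds multiplied points.
; GetAttachPoint exposes the Arrow's world transform.
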(event `self.Box.OnComponentBeginOverlap`
  (params (OverlappedComponent :type "PrimitiveComponent Object Reference") (OtherActor :type "Actor Object Reference") (OtherComp :type "PrimitiveComponent Object Reference") (OtherBodyIndex :type Integer) (bFromSweep :type Boolean) (SweepResult :type "HitResult Structure (by ref)"))
  ;[1 1 1] Extend Floor
  (bind _asbp_runner_game_mode (cast `/Game/Runner/Blueprints/BP_RunnerGameMode` (`GameplayStatics.GetGameMode`)))
  (`/Game/Runner/Blueprints/BP_RunnerGameMode.Extend Floor` _asbp_runner_game_mode)
  ;[1 1 1] Change Speed
  (bind _asbp_runner_character (cast `/Game/Runner/Blueprints/CharacterBPs/BP_RunnerCharacter` (`GameplayStatics.GetPlayerCharacter` 0)))
  (bind _charactermovement (`Character.CharacterMovement` _asbp_runner_character))
  (bind _output_get (set `CharacterMovementComponent.MaxWalkSpeed` (`KismetMathLibrary.FClamp` (* (`CharacterMovementComponent.MaxWalkSpeed` _charactermovement) 1.01) 700.0 1500.0) _charactermovement))
  (`KismetSystemLibrary.PrintString` (`KismetStringLibrary.Conv_DoubleToString` _output_get))
  ;[1 1 1] Set Current Score
  (bind _asbp_runner_game_mode_2 (cast `/Game/Runner/Blueprints/BP_RunnerGameMode` (`GameplayStatics.GetGameMode`)))
  (set `/Game/Runner/Blueprints/BP_RunnerGameMode.Current Points` (+ (* (`/Game/Runner/Blueprints/BP_RunnerGameMode.Points Multi` _asbp_runner_game_mode_2) 1) (`/Game/Runner/Blueprints/BP_RunnerGameMode.Current Points` _asbp_runner_game_mode_2)) _asbp_runner_game_mode_2))

(fn `Coin Spawn Points`
  (for _array_element (`self.Lane Position`)
    (for _index (range 6)
      (bind _returnvalue (`AddComponent|NODE_AddArrowComponent-2` :`RelativeTransform` (`KismetMathLibrary.MakeTransform` (`KismetMathLibrary.MakeVector` (* _index 75.0) _array_element))))
      (`ArrowComponent.SetArrowColor` _returnvalue (struct :`R` 0.870475 :`G` 0.328016 :`B` 1.0 :`A` 1.0))
      (`KismetArrayLibrary.Array_Add` (`self.CSpawnPoints`) (`SceneComponent.K2_GetComponentToWorld` _returnvalue)))))

(fn `Get AttachPoint`
  (returns (ReturnValue :type "Transform Structure"))
  (return (`SceneComponent.K2_GetComponentToWorld` (`self.Arrow`))))

(fn `PowerUps Spawn Points`
  (for _array_element (`self.Lane Position`)
    (for _index (range 1 3)
      (bind _returnvalue (`AddComponent|NODE_AddArrowComponent-3` :`RelativeTransform` (`KismetMathLibrary.MakeTransform` (`KismetMathLibrary.MakeVector` (* _index 1200.0) _array_element))))
      (`ArrowComponent.SetArrowColor` _returnvalue (struct :`G` 0.050913 :`B` 1.0 :`A` 1.0))
      (`KismetArrayLibrary.Array_Add` (`self.PSpawn Points`) (`SceneComponent.K2_GetComponentToWorld` _returnvalue)))))

(fn `Setup Spawn Points`
  (for _array_element (`self.Lane Position`)
    (for _index (range 2)
      (bind _returnvalue (`AddComponent|NODE_AddArrowComponent-0` :`RelativeTransform` (`KismetMathLibrary.MakeTransform` (`KismetMathLibrary.MakeVector` (* _index 1200.0) _array_element))))
      (`KismetArrayLibrary.Array_Add` (`self.Spawn Points`) (`SceneComponent.K2_GetComponentToWorld` _returnvalue)))))

(fn `Spawn Coins`
  (locals (`Random Spawn Point` :type "Array of Transform Structure"))
  (bind _output_get (set `local.Random Spawn Point` (`self.CSpawnPoints`)))
  (`KismetArrayLibrary.Array_Shuffle` _output_get)
  (for _index (range (+ (`KismetMathLibrary.RandomIntegerInRange` 2 5) 1))
    (switch `int` 0
      (:`0`
        (`AddComponent|NODE_AddChildActorComponent-4` :`RelativeTransform` (`KismetMathLibrary.MakeRelativeTransform` (`|GetArrayItem` (`local.Random Spawn Point`) _index) (`self.GetTransform`)))))))

(fn `Spawn Obstacles`
  (locals (`Random Spawn Point` :type "Array of Transform Structure"))
  (bind _output_get (set `local.Random Spawn Point` (`self.Spawn Points`)))
  (`KismetArrayLibrary.Array_Shuffle` _output_get)
  (for _index (range (+ (`KismetMathLibrary.RandomIntegerInRange` 0 1) 1))
    (switch `int` (`KismetMathLibrary.RandomIntegerInRange` 0 1)
      (:`0`
        (bind _returnvalue (`KismetMathLibrary.MakeRelativeTransform` (`|GetArrayItem` (`local.Random Spawn Point`) _index) (`self.GetTransform`)))
        (`AddComponent|NODE_AddChildActorComponent-0` :`RelativeTransform` _returnvalue))
      (:`1`
        (`AddComponent|NODE_AddChildActorComponent-1` :`RelativeTransform` _returnvalue)))))

(fn `Spawn PowerUps`
  (locals (`Random Spawn Point` :type "Array of Transform Structure"))
  (bind _asbp_runner_game_mode (cast `/Game/Runner/Blueprints/BP_RunnerGameMode` (`GameplayStatics.GetGameMode`)))
  (if (> (`/Game/Runner/Blueprints/BP_RunnerGameMode.Floor Count` _asbp_runner_game_mode) 5)
    (bind _output_get (set `local.Random Spawn Point` (`self.PSpawn Points`)))
    (`KismetArrayLibrary.Array_Shuffle` _output_get)
    (switch `int` 0
      (:`0`
        (`AddComponent|NODE_AddChildActorComponent-5` :`RelativeTransform` (`KismetMathLibrary.MakeRelativeTransform` (`|GetArrayItem` (`local.Random Spawn Point`)) (`self.GetTransform`)))
        (set `/Game/Runner/Blueprints/BP_RunnerGameMode.Floor Count` 0 _asbp_runner_game_mode)))))

(fn `UserConstructionScript`
  (`self.Setup Spawn Points`)
  (`self.Spawn Obstacles`)
  (`self.Coin Spawn Points`)
  (`self.Spawn Coins`)
  (`self.PowerUps Spawn Points`)
  (`self.Spawn PowerUps`))